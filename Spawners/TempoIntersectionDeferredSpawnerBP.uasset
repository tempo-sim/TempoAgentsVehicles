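; Mass traffic spawner Blueprint that can defer its spawning until traffic intersections are set up.
; On BeginPlay it uses its assigned intersection spawner, or the first one found in the world, and binds to that spawner's spawning-finished event.
; The intersections-fully-setup handler calls DoSpawning when SpawnAfterIntersections is enabled.
; When its own despawning finishes, it clears all lanes through the MassTraffic subsystem.
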(event `self.ReceiveBeginPlay`
  (`parent.ReceiveBeginPlay`)
  (add `self.OnDespawningFinishedEvent` (delegate `OnDespawningFinished`))
  (if (not (`KismetSystemLibrary.IsValid` (`self.IntersectionSpawner`)))
    (bind _outactors (`GameplayStatics.GetAllActorsOfClass` "/Game/TempoAgentsVehicles/Spawners/TempoIntersectionSpawnerBP.TempoIntersectionSpawnerBP_C"))
    (if (`KismetArrayLibrary.Array_IsNotEmpty` _outactors)
      (set `self.IntersectionSpawner` (`|GetArrayItem` _outactors))
      (add `self.OnSpawningFinishedEvent` (`self.IntersectionSpawner`) (`|CreateDelegate` :!event `OnIntersectionsFullySetup`) :!label _label))
    (else
      (goto _label))))

(event `OnDespawningFinished`
  (`MassTrafficSubsystem.ClearAllTrafficLanes` (subsystem `MassTrafficSubsystem`)))

(event `OnIntersectionsFullySetup`
  (if (`self.SpawnAfterIntersections`)
    (`self.DoSpawning`)))

(fn `UserConstructionScript`)